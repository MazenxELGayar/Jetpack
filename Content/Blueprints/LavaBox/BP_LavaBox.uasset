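; BP_LavaBox is a kill volume made of a lava floor, a ceiling and four walls that kills actors touching it.
; Begin overlap on any of the six components routes to a shared KillActor function.
; KillActor sends a DieInstantly interface message to the overlapping actor, passing that actor's transform and the box as instigator.
; The forwarded sweep hit is unused.
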(event `self.Ceiling.OnComponentBeginOverlap`
  (params (OverlappedComponent :type "PrimitiveComponent Object Reference") (OtherActor :type "Actor Object Reference") (OtherComp :type "PrimitiveComponent Object Reference") (OtherBodyIndex :type Integer) (bFromSweep :type Boolean) (SweepResult :type "HitResult Structure (by ref)"))
  (`self.KillActor` OtherActor SweepResult))

(event `self.LavaFloor.OnComponentBeginOverlap`
  (params (OverlappedComponent :type "PrimitiveComponent Object Reference") (OtherActor :type "Actor Object Reference") (OtherComp :type "PrimitiveComponent Object Reference") (OtherBodyIndex :type Integer) (bFromSweep :type Boolean) (SweepResult :type "HitResult Structure (by ref)"))
  (`self.KillActor` OtherActor SweepResult))

(event `self.Wall1.OnComponentBeginOverlap`
  (params (OverlappedComponent :type "PrimitiveComponent Object Reference") (OtherActor :type "Actor Object Reference") (OtherComp :type "PrimitiveComponent Object Reference") (OtherBodyIndex :type Integer) (bFromSweep :type Boolean) (SweepResult :type "HitResult Structure (by ref)"))
  (`self.KillActor` OtherActor SweepResult))

(event `self.Wall2.OnComponentBeginOverlap`
  (params (OverlappedComponent :type "PrimitiveComponent Object Reference") (OtherActor :type "Actor Object Reference") (OtherComp :type "PrimitiveComponent Object Reference") (OtherBodyIndex :type Integer) (bFromSweep :type Boolean) (SweepResult :type "HitResult Structure (by ref)"))
  (`self.KillActor` OtherActor SweepResult))

(event `self.Wall3.OnComponentBeginOverlap`
  (params (OverlappedComponent :type "PrimitiveComponent Object Reference") (OtherActor :type "Actor Object Reference") (OtherComp :type "PrimitiveComponent Object Reference") (OtherBodyIndex :type Integer) (bFromSweep :type Boolean) (SweepResult :type "HitResult Structure (by ref)"))
  (`self.KillActor` OtherActor SweepResult))

(event `self.Wall4.OnComponentBeginOverlap`
  (params (OverlappedComponent :type "PrimitiveComponent Object Reference") (OtherActor :type "Actor Object Reference") (OtherComp :type "PrimitiveComponent Object Reference") (OtherBodyIndex :type Integer) (bFromSweep :type Boolean) (SweepResult :type "HitResult Structure (by ref)"))
  (`self.KillActor` OtherActor SweepResult))

(fn `KillActor`
  (params (OtherActor :type "Actor Object Reference") (Hit :type "HitResult Structure (by ref)"))
  (message `/Game/Blueprints/Interfaces/BPI_GetHurt.DieInstantly` OtherActor (`self.GetTransform` OtherActor) self))

(fn `UserConstructionScript`)