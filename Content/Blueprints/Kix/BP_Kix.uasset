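; BP_Kix is the Kix character Blueprint, providing jetpack thruster feedback and fuel management.
; Toggling thrusters switches the left and right effects and plays start or stop sounds, with a reused, attached loop that fades in.
; Drain and restore events adjust fuel by delta time, clamped to its maximum.
; Getters expose fuel, move input and a start check that can require a recharge threshold.
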(event `/Game/Blueprints/Interfaces/BPI_Thrusters.ActivateOrDecativateThrusters`
  (params (Activate :type Boolean))
  (`self.ActivateOrDecativateThrustersByBoolean` Activate))

(event `/Game/Blueprints/Interfaces/BPI_Thrusters.DrainJettFuel`
  (`self.ConsumeJettFuel`))

(event `/Game/Blueprints/Interfaces/BPI_Thrusters.RestoreJettFuelWhenNotFlying`
  (`self.RestoreJettFuel`))

(fn `ActivateOrDecativateThrustersByBoolean`
  (params (Activate :type Boolean))
  (`ActorComponent.SetActive` (`self.Thruster_L_Effect`) Activate false)
  (`ActorComponent.SetActive` (`self.Thruster_R_Effect`) Activate false)
  (if (`local.Activate`)
    (`self.PlayThrustersSounds`)
    (else
      (`self.PlayEndThrustersSoundsAndStopStartingSound`))))

(fn `CanStartJettFuel`
  (params (WaitRechargeLimit :type Boolean))
  (returns (CanStartJettFuelResult :type Boolean))
  (return (> (`self.JettFuel`) (`KismetMathLibrary.SelectFloat` (`self.JettFuelStartLimit`) 0.0 (`local.WaitRechargeLimit`)))))

(fn `ConsumeJettFuel`
  (set `self.JettFuel` (`KismetMathLibrary.FClamp` (- (`self.JettFuel`) (* (`self.JettFuelDrainRate`) (`GameplayStatics.GetWorldDeltaSeconds`))) 0.0 (`self.MaxJettFuel`))))

(fn `GetFlyingMultiplier`
  (returns (FlyingMaxAccelerationMultiplier :type "Float (double-precision)"))
  (return 5e-05))

(fn `GetFuelStartThresold`
  (returns (JettFuelStartLimit :type "Float (double-precision)") (JettFuelStartLimitPercentage :type "Float (double-precision)"))
  (return (`self.JettFuelStartLimit`) (/ (`self.JettFuelStartLimit`) (`self.MaxJettFuel`))))

(fn `GetJettFuel`
  (returns (JettFuel :type "Float (double-precision)"))
  (return (`self.JettFuel`)))

(fn `GetMaxJettFuel`
  (returns (JettFuel :type "Float (double-precision)"))
  (return (`self.MaxJettFuel`)))

(fn `GetMoveInput`
  (returns (InputActionValue :type "Vector2D Structure"))
  (return (`|GetInputActionValue`)))

(fn `PlayEndThrustersSoundsAndStopStartingSound`
  (`self.StopThrusterLoopingSound`)
  (bind _returnvalue (`GameplayStatics.SpawnSoundAtLocation` "/Game/Assets/Sounds/Thrusters/SW_Jetpack_Stop_01.SW_Jetpack_Stop_01" (`self.K2_GetActorLocation`) (struct) 1.0 1.0 0.0 null null))
  (`AudioComponent.FadeOut` _returnvalue 0.55 0.0 "Linear"))

(fn `PlayThrustersSounds`
  (`self.PlayThrusterStartSound`)
  (`/Engine/EditorBlueprintResources/StandardMacros.IsValid` (`self.LoopingThrusterSound`)
    (:`Is Valid`
      (`AudioComponent.Play` (`self.LoopingThrusterSound`) 0.0)
      (`AudioComponent.FadeIn` (`self.LoopingThrusterSound`) 0.35 1.0 0.0 "Linear"))
    (:`Is Not Valid`
      (bind _returnvalue (`GameplayStatics.SpawnSoundAttached` "/Game/Assets/Sounds/Thrusters/MS_ThrusterLoop.MS_ThrusterLoop" (`self.CapsuleComponent`) "None" (0.0 0.0 0.0) (struct) "KeepRelativeOffset" false 1.0 1.0 0.0 null null false))
      (bind _output_get (set `self.LoopingThrusterSound` _returnvalue))
      (`AudioComponent.FadeIn` _output_get 0.35 1.0 0.0 "Linear"))))

(fn `PlayThrusterStartSound`
  (bind _returnvalue (`GameplayStatics.SpawnSoundAtLocation` "/Game/Assets/Sounds/Thrusters/SW_Jetpack_Start_01.SW_Jetpack_Start_01" (`self.K2_GetActorLocation`) (struct) 1.0 1.0 0.0 null null))
  (`AudioComponent.FadeOut` _returnvalue 1.0 0.0 "Linear"))

(fn `RestoreJettFuel`
  (set `self.JettFuel` (`KismetMathLibrary.FClamp` (+ (`self.JettFuel`) (* (`self.JettFuelRestoreRate`) (`GameplayStatics.GetWorldDeltaSeconds`))) 0.0 (`self.MaxJettFuel`))))

(fn `StopThrusterLoopingSound`
  (bind _loopingthrustersound (`self.LoopingThrusterSound`)
    (:`then`
      (`AudioComponent.Stop` _loopingthrustersound))
    (:`else`)))

(fn `UserConstructionScript`)