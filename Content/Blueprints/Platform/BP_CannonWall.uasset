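; BP_CannonWall is a destructible wall with a child-actor BP_Cannon and its own HP.
; Damage, instant-death and heal events lower HP, raise it without a MaxHP clamp, or destroy the wall with an explosion effect.
; Each change prints a debug message to screen, naming the killer on destruction.
; Getters expose the cannon and the HP, MaxHP and health percentage.
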(event `self.ReceiveBeginPlay`)

(event `/Game/Blueprints/Interfaces/BPI_GetHurt.GetHurt`
  (params (Damage :type Integer) (KillInstant :type Boolean) (SpawnTransform :type "Transform Structure") (Intestigator :type "Actor Object Reference"))
  ;[0.008758 0.151 0.06274] GetHurt
  (`self.HurtOrDestroyWall` Damage KillInstant SpawnTransform Intestigator))

(event `/Game/Blueprints/Interfaces/BPI_GetHurt.DieInstantly`
  (params (SpawnTransform :type "Transform Structure") (Intestigator :type "Actor Object Reference"))
  ;[0.008758 0.151 0.06274] DieInstantly
  (`self.DestroyWall` SpawnTransform Intestigator))

(event `/Game/Blueprints/Interfaces/BPI_GetHurt.Heal`
  (params (HealAmount :type Integer) (Intestigator :type "Actor Object Reference"))
  ;[0.008758 0.151 0.06274] HealPlayer
  (`self.HealWall` HealAmount))

(fn `DecreaseWallHp`
  (params (Damage :type Integer) (SpawnTransform :type "Transform Structure") (Hurter :type "Actor Object Reference"))
  (set `self.HP` (- (`self.HP`) Damage))
  (`self.PrintHealLogs` " was damaged to " (struct :`R` 0.348958 :`A` 1.0)))

(fn `DestroyWall`
  (params (SpawnTransform :type "Transform Structure") (Killer :type "Actor Object Reference"))
  (locals (isPlayerControlled :type Boolean) (chars :type "Array of Object Object Reference"))
  (`|SpawnActorFromClass` "/Game/StarterContent/Blueprints/Blueprint_Effect_Explosion.Blueprint_Effect_Explosion_C" SpawnTransform "Undefined" "MultiplyWithRoot" null null)
  (`self.K2_DestroyActor`)
  (`KismetSystemLibrary.PrintString` (`KismetStringLibrary.Concat_StrStr` (`KismetSystemLibrary.GetDisplayName` self) " was Destroyed by " (`KismetSystemLibrary.GetDisplayName` Killer))))

(fn `GetBpCannon`
  (returns (BPCannon :type "/Game/Blueprints/Cannon/BP_Cannon Object Reference"))
  (bind _asbp_cannon (cast `/Game/Blueprints/Cannon/BP_Cannon` (`ChildActorComponent.ChildActor` (`self.BP_Cannon`))))
  (return _asbp_cannon))

(fn `GetHP`
  (returns (HP :type "Float (double-precision)") (MaxHP :type "Float (double-precision)") (Percent :type "Float (double-precision)"))
  (bind _hp (`self.HP`))
  (bind _maxhp (`self.MaxHP`))
  (return _hp _maxhp (`KismetMathLibrary.SafeDivide` _hp _maxhp)))

(fn `HealWall`
  (params (HealAmount :type Integer))
  (set `self.HP` (+ HealAmount (`self.HP`)))
  (`self.PrintHealLogs` " was Healed to " (struct :`R` 0.008758 :`G` 0.151042 :`B` 0.062743 :`A` 1.0)))

(fn `HurtOrDestroyWall`
  (params (Damage :type Integer) (KillInstant :type Boolean) (SpawnTransform :type "Transform Structure") (Intestigator :type "Actor Object Reference"))
  (if (or (>= Damage (`self.HP`)) KillInstant)
    (`self.DestroyWall` SpawnTransform Intestigator)
    (else
      (`self.DecreaseWallHp` Damage SpawnTransform Intestigator))))

(fn `PrintHealLogs`
  (params (EffectString :type String :default " was Healed to ") (TextColor :type "LinearColor Structure"))
  (bind _returnvalue (`KismetSystemLibrary.GetDisplayName` self))
  (`KismetSystemLibrary.PrintString` (`KismetStringLibrary.Concat_StrStr` _returnvalue EffectString (`KismetStringLibrary.Conv_IntToString` (`KismetMathLibrary.FTrunc` (`self.HP`)))) true true TextColor 2.0 (`KismetStringLibrary.Conv_StringToName` (`KismetStringLibrary.Concat_StrStr` _returnvalue "Heal"))))

(fn `UserConstructionScript`)