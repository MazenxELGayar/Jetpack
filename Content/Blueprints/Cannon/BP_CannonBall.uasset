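; Cannonball projectile actor that explodes on its first overlap and damages actors around the impact.
; The overlap's sweep result drives a sequence that destroys the ball and spawns a Niagara fire explosion and sound at the hit, aligned to its normal for the effect.
; A sphere overlap filtered by object type then sends each actor found GetHurtMessage with flat damage, the impact transform and the ball as instigator.
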(event `self.cannonball.OnComponentBeginOverlap`
  (params (OverlappedComponent :type "PrimitiveComponent Object Reference") (OtherActor :type "Actor Object Reference") (OtherComp :type "PrimitiveComponent Object Reference") (OtherBodyIndex :type Integer) (bFromSweep :type Boolean) (SweepResult :type "HitResult Structure (by ref)"))
  (`|ExecutionSequence`
    (:`then_0`
      (`self.DestroyAndExplode` SweepResult))
    (:`then_1`
      (`self.FindActorsNearExplosionAndHurtThem` SweepResult))))

(fn `DestroyAndExplode`
  (params (Hit :type "HitResult Structure (by ref)"))
  (bind (_bblockinghit _binitialoverlap _time _distance _location _impactpoint _normal) (`GameplayStatics.BreakHitResult` Hit))
  (`self.K2_DestroyActor`)
  (`NiagaraFunctionLibrary.SpawnSystemAtLocation` "/Game/Assets/Effects/Projectiles/FireExplosion/NS_FireExplosion.NS_FireExplosion" _location (`KismetMathLibrary.MakeRotFromX` _normal) (100.0 100.0 100.0))
  (`GameplayStatics.SpawnSoundAtLocation` "/Game/StarterContent/Audio/Explosion01.Explosion01" _location (struct) 1.0 1.0 0.0 null null))

(fn `FindActorsNearExplosionAndHurtThem`
  (params (Hit :type "HitResult Structure (by ref)"))
  (bind (_hit_bblockinghit _hit_binitialoverlap _hit_time _hit_distance _hit_location _hit_impactpoint _hit_normal) (`GameplayStatics.BreakHitResult` (`local.Hit`)))
  (bind (_hit_bblockinghit_2 _hit_binitialoverlap_2 _hit_time_2 _hit_distance_2 _hit_location_2) (`GameplayStatics.BreakHitResult` (`local.Hit`)))
  (bind _outactors (`KismetSystemLibrary.SphereOverlapActors` _hit_location_2 (`self.ExplosionRadius`) (`self.AffectedTypes`) null (`|MakeArray` self :!type "Actor Object Reference")))
  (for _array_element _outactors
    (message `/Game/Blueprints/Interfaces/BPI_GetHurt.GetHurt` _array_element (`self.CannonBallDamage`) false (`KismetMathLibrary.MakeTransform` _hit_location (`KismetMathLibrary.MakeRotFromX` _hit_normal)) self)))

(fn `UserConstructionScript`)