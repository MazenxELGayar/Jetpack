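; Cannon actor that targets the closest BP_Bot and fires BP_CannonBall projectiles at it.
; On BeginPlay, StoreTargetPawn gathers all bots and caches the nearest by distance, with an optional distance reset and on-screen debug prints.
; SpawnCannonBall, not called within this Blueprint, rotates the actor toward that cached target, then plays an explosion sound and spawns the ball at the tube's socket.
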(event `self.ReceiveBeginPlay`
  (`self.StoreTargetPawn` false))

(fn `GetClosesBotFromArray`
  (for _array_element (`self.Enemies`)
    (bind _returnvalue (`self.GetLocationFromCannon` _array_element))
    (if (< _returnvalue (`self.ClosestEnemyDistance`))
      (`|ExecutionSequence`
        (:`then_0`
          (set `self.ClosestEnemyDistance` _returnvalue))
        (:`then_1`
          (set `self.ClosestEnemy` _array_element)))))
  (`/Engine/EditorBlueprintResources/StandardMacros.IsValid` (`self.ClosestEnemy`)
    (:`Is Valid`
      (`KismetSystemLibrary.PrintString` (`KismetStringLibrary.Concat_StrStr` "Closest Pawn: " (`KismetSystemLibrary.GetDisplayName` (`self.ClosestEnemy`)) ", At Index " (`KismetStringLibrary.Conv_IntToString` 0) ", Distance: " (`KismetStringLibrary.Conv_DoubleToString` (`self.ClosestEnemyDistance`))) true true (struct :`G` 0.66 :`B` 1.0 :`A` 1.0) 4.0))
    (:`Is Not Valid`
      (`KismetSystemLibrary.PrintString` "NO MORE PAWNS TO HIT" true true (struct :`R` 0.056602 :`G` 0.088133 :`B` 1.0 :`A` 1.0) 234343.0 "NO MORE PAWNS TO HIT"))))

(fn `GetLocationFromCannon`
  (params (Actor :type "Actor Object Reference"))
  (returns (ReturnValue :type "Float (double-precision)"))
  (`/Engine/EditorBlueprintResources/StandardMacros.IsValid` Actor
    (:`Is Valid`
      (return (`KismetMathLibrary.Vector_Distance` (`self.K2_GetActorLocation` Actor) (`self.CannonLocation`))))))

(fn `RotateToEnemyIfValid`
  (locals (NewRotationToEnemy :type "Rotator Structure" :default (struct)))
  (bind _closestenemy (`self.ClosestEnemy`)
    (:`then`
      (`self.K2_SetActorRotation` (`KismetMathLibrary.RInterpTo` (`self.K2_GetActorRotation`) (`KismetMathLibrary.FindLookAtRotation` (`self.K2_GetActorLocation`) (`self.K2_GetActorLocation` _closestenemy)) (`GameplayStatics.GetWorldDeltaSeconds`))))
    (:`else`)))

(fn `SpawnCannonBall`
  (bind _returnvalue (`SceneComponent.GetSocketTransform` (`self.SM_Cannon_Tube`) (`self.CannonBallSpawnSocketName`) "RTS_World"))
  (`self.RotateToEnemyIfValid`)
  (`GameplayStatics.SpawnSoundAtLocation` "/Game/StarterContent/Audio/Explosion01.Explosion01" (.location _returnvalue) (struct) 1.0 1.0 0.0 null null)
  (`|SpawnActorFromClass` "/Game/Blueprints/Cannon/BP_CannonBall.BP_CannonBall_C" _returnvalue "AlwaysSpawn" "MultiplyWithRoot" self null))

(fn `StoreTargetPawn`
  (params (resetClosestDistance :type Boolean))
  (if resetClosestDistance
    (set `self.ClosestEnemyDistance` 999999999999999.0))
  (`KismetSystemLibrary.PrintString` "Store Target Pawn Called" true true (struct :`G` 0.66 :`B` 1.0 :`A` 1.0) 3.0)
  (`|ExecutionSequence`
    (:`then_0`
      (set `self.CannonLocation` (`self.K2_GetActorLocation`)))
    (:`then_1`
      (bind _outactors (`GameplayStatics.GetAllActorsOfClass` "/Game/Blueprints/Drone/BP_Bot.BP_Bot_C"))
      (set `self.Enemies` _outactors)
      (`self.GetClosesBotFromArray`))))

(fn `UserConstructionScript`)