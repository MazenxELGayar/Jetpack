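; BP_BlasterBeam is a blaster projectile, filed under Drone, that damages what it hits.
; It binds to BeamMesh's component hit event on BeginPlay and ignores hits on other blaster beams.
; On any other hit, ShowFXAndDestroyBeam spawns a Niagara burst, destroys the beam and returns the hit actor.
; That actor then receives GetHurtMessage with the beam's damage and a transform aligned to the impact normal.
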(event `self.ReceiveBeginPlay`
  (`|ExecutionSequence`
    (:`then_1`
      (add `PrimitiveComponent.OnComponentHit` (`self.BeamMesh`) (delegate `OnComponentHit_Event`)))))

(event `OnComponentHit_Event`
  (params (HitComponent :type "PrimitiveComponent Object Reference") (OtherActor :type "Actor Object Reference") (OtherComp :type "PrimitiveComponent Object Reference") (NormalImpulse :type "Vector Structure") (Hit :type "HitResult Structure (by ref)"))
  (bind (_bblockinghit _binitialoverlap _time _distance _location _impactpoint _normal) (`GameplayStatics.BreakHitResult` Hit))
  (cast `/Game/Blueprints/Drone/BP_BlasterBeam` OtherActor
    (:`CastFailed`
      (bind _hitactor (`self.ShowFXAndDestroyBeam` Hit))
      (message `/Game/Blueprints/Interfaces/BPI_GetHurt.GetHurt` _hitactor (`self.BlasterBeamDamage`) false (`KismetMathLibrary.MakeTransform` _impactpoint (`KismetMathLibrary.Conv_VectorToRotator` _normal)) null))))

(fn `ShowFXAndDestroyBeam`
  (params (Hit :type "HitResult Structure (by ref)"))
  (returns (HitActor :type "Actor Object Reference"))
  (bind (_bblockinghit _binitialoverlap _time _distance _location _impactpoint _normal _impactnormal _physmat _hitactor) (`GameplayStatics.BreakHitResult` Hit))
  (`NiagaraFunctionLibrary.SpawnSystemAtLocation` "/Game/Assets/FX/NS_BeamBurst.NS_BeamBurst" _location (`KismetMathLibrary.MakeRotFromX` _normal))
  (`self.K2_DestroyActor`)
  (return _hitactor))

(fn `UserConstructionScript`)