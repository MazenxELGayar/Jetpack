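; Pressure plate Blueprint that fires its attached cannons when pressed.
; AttachCannonToButton adds valid cannons to the CannonsAttached set.
; OnPress runs the parent logic, then calls SpawnCannonBall on each valid cannon and removes invalid entries from the set during the loop.
; OnUnPress only calls the parent implementation.
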(fn `AttachCannonToButton`
  (params (BP_Cannon :type "/Game/Blueprints/Cannon/BP_Cannon Object Reference"))
  (bind _bp_cannon (`local.BP_Cannon`)
    (:`then`
      (`BlueprintSetLibrary.Set_Add` (`self.CannonsAttached`) _bp_cannon))
    (:`else`)))

(fn `OnPress`
  (`parent.OnPress`)
  (bind _valuepin (`|SetForEach` (`self.CannonsAttached`))
    (:`then`
      (`/Engine/EditorBlueprintResources/StandardMacros.IsValid` _valuepin
        (:`Is Valid`
          (`/Game/Blueprints/Cannon/BP_Cannon.SpawnCannonBall` _valuepin))
        (:`Is Not Valid`
          (`BlueprintSetLibrary.Set_Remove` (`self.CannonsAttached`) _valuepin))))))

(fn `OnUnPress`
  (`parent.OnUnPress`))

(fn `UserConstructionScript`
  (`parent.UserConstructionScript`))