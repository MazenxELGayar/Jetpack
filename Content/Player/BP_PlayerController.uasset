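; Player controller that handles movement and camera look for the controlled pawn through Enhanced Input.
; On BeginPlay it adds the IMC_Kix mapping context.
; Look input drives controller yaw and pitch through LookAround.
; Move input is sent as forced input vectors straight to the pawn's movement component, along the control rotation's forward and right vectors, so forward movement follows camera pitch.
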(event `self.ReceiveBeginPlay`
  (`EnhancedInputSubsystemInterface.AddMappingContext` (subsystem `EnhancedInputLocalPlayerSubsystem`) "/Game/Input/IMC_Kix.IMC_Kix" 0 (struct)))

(event `EnhancedInput|/Game/Input/inputAction/IA_Look`
  (params (ActionValue :type "Vector2D Structure") (ElapsedSeconds :type "Float (double-precision)") (TriggeredSeconds :type "Float (double-precision)") (InputAction :type "InputAction Object Reference" :default "/Game/Input/inputAction/IA_Look.IA_Look"))
  (:`Triggered`
    (`self.LookAround` ActionValue)))

(event `EnhancedInput|/Game/Input/inputAction/IA_Move`
  (params (ActionValue :type "Vector2D Structure") (ElapsedSeconds :type "Float (double-precision)") (TriggeredSeconds :type "Float (double-precision)") (InputAction :type "InputAction Object Reference" :default "/Game/Input/inputAction/IA_Move.IA_Move"))
  (bind _returnvalue (`self.GetControlRotation`))
  (bind _returnvalue_x (`KismetMathLibrary.BreakVector2D` (`|GetInputActionValue`)))
  (bind (_returnvalue_x_2 _returnvalue_y) (`KismetMathLibrary.BreakVector2D` (`|GetInputActionValue`)))
  (bind _returnvalue_2 (`Pawn.GetMovementComponent` (`self.K2_GetPawn`)))
  (:`Triggered`
    (`|ExecutionSequence`
      (:`then_0`
        (`PawnMovementComponent.AddInputVector` _returnvalue_2 (* _returnvalue_y (`KismetMathLibrary.GetForwardVector` _returnvalue)) true))
      (:`then_1`
        (`PawnMovementComponent.AddInputVector` _returnvalue_2 (* (`KismetMathLibrary.GetRightVector` _returnvalue) _returnvalue_x) true)))))

(fn `LookAround`
  (params (Movement :type "Vector2D Structure"))
  (bind (_x _y) (`KismetMathLibrary.BreakVector2D` Movement))
  (`|ExecutionSequence`
    (:`then_0`
      (`self.AddYawInput` _x))
    (:`then_1`
      (`self.AddPitchInput` _y))))

(fn `UserConstructionScript`)